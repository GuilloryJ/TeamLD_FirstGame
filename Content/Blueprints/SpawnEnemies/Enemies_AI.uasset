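; Enemy AI Blueprint that chases the player and triggers an attack on any actor overlap.
; A Tick accumulator throttles updates to roughly every 0.4 seconds, issuing SimpleMoveToLocation toward the player pawn.
; The same update checks velocity to play looping Run, or Idle after a delay, directly on the mesh.
; Attacks go through the Enemies_Anim instance cached at BeginPlay.
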(event `self.ReceiveBeginPlay`
  (bind _asenemies_anim (cast `/Game/Blueprints/SpawnEnemies/Enemies_Anim` (`SkeletalMeshComponent.GetAnimInstance` (`self.Mesh`)))))

(event `self.ReceiveActorBeginOverlap`
  (params (OtherActor :type "Actor Object Reference"))
  (`/Game/Blueprints/SpawnEnemies/Enemies_Anim.Attack!` (stale `self.ReceiveBeginPlay` _asenemies_anim)))

(event `self.ReceiveTick`
  (params (DeltaSeconds :type "Float (single-precision)"))
  (bind _mesh (`self.Mesh`))
  (set `self.EventTick` (+ DeltaSeconds (`self.EventTick`)))
  (if (>= (`self.EventTick`) 0.4)
    (set `self.EventTick` (`self.EventTickTime`))
    (`|ExecutionSequence`
      (:`then_0`
        (`NavigationSystem.SimpleMoveToLocation` (`self.GetController` self) (`self.K2_GetActorLocation` (`GameplayStatics.GetPlayerPawn` 0))))
      (:`then_1`
        (set `self.Speed` (`KismetMathLibrary.VSize` (`self.GetVelocity`)))
        (if (>= (`self.Speed`) 5.0)
          (`SkeletalMeshComponent.PlayAnimation` _mesh "/Game/Animations/Run.Run" true)
          (else
            (`KismetSystemLibrary.Delay` 2.64)
            (`SkeletalMeshComponent.PlayAnimation` _mesh "/Game/Animations/Idle.Idle" true)))))))

(event `Run`)

(fn `UserConstructionScript`)