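; MyHUD is a HUD Blueprint that draws the player character's health value on screen.
; On BeginPlay it finds all MyCharacter actors and stores the cast result, keeping the last one found.
; DrawHUD then prints that character's HPStart variable as scaled white text near the bottom-right corner of the viewport.
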(event `self.ReceiveDrawHUD`
  (params (SizeX :type Integer) (SizeY :type Integer))
  (`self.DrawText` (`KismetStringLibrary.Conv_DoubleToString` (`/Game/Blueprints/MyCharacter.HP_start` (stale `self.ReceiveBeginPlay` _asmy_character))) (struct :`R` 1.0 :`G` 1.0 :`B` 1.0 :`A` 1.0) (`KismetMathLibrary.Conv_IntToDouble` (- SizeX 100)) (`KismetMathLibrary.Conv_IntToDouble` (- SizeY 100)) null 2.0))

(event `self.ReceiveBeginPlay`
  (bind _outactors (`GameplayStatics.GetAllActorsOfClass` "/Game/Blueprints/MyCharacter.MyCharacter_C"))
  (for _array_element _outactors
    (bind _asmy_character (cast `/Game/Blueprints/MyCharacter` _array_element))))

(event `self.ReceiveActorBeginOverlap`
  (params (OtherActor :type "Actor Object Reference")))

(event `self.ReceiveTick`
  (params (DeltaSeconds :type "Float (single-precision)")))

(fn `UserConstructionScript`)